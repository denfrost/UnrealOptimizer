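; BP_Character is a character Blueprint with a floating 3D label that displays render-visibility status from its OptimizerActor.
; Each Tick, it rotates the Widget component to face the player camera.
; It then casts the widget to UI_3dLabel and writes the DelayRender result of OptimizerActor's WasRecentlyRendered check, using a short tolerance, into the label text.
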(event `self.ReceiveBeginPlay`)

(event `self.ReceiveTick`
  (params (DeltaSeconds :type "Float (single-precision)"))
  (bind _widget (`self.Widget`))
  (`|ExecutionSequence`
    (:`then_1`
      (`SceneComponent.K2_SetWorldRotation` _widget (`KismetMathLibrary.FindLookAtRotation` (`SceneComponent.K2_GetComponentLocation` _widget) (`PlayerCameraManager.GetCameraLocation` (`GameplayStatics.GetPlayerCameraManager` 0))) false false)
      (bind _asui_3d_label (cast `/UnrealOptimizer/UI_3dLabel` (`WidgetComponent.GetUserWidgetObject` (`self.Widget`))))
      (set `/UnrealOptimizer/UI_3dLabel.3dLabelText` (`KismetTextLibrary.Conv_StringToText` (`KismetStringLibrary.Conv_DoubleToString` (`OptimizerActorComponent.WasRecentlyRendered` (`self.OptimizerActor`) 0.05))) _asui_3d_label))))

(fn `UserConstructionScript`)