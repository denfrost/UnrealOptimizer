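; BP_ActorEmpty is an actor that prints visibility debug output for its OptimizerActor and Cube.
; OptimizerActor's OnCheckVisible event stores the flag in Visible and prints it with the actor name and game time.
; Every Tick prints whether OptimizerActor reports Cube as recently rendered, alongside the stored flag, for on-screen comparison.
; A SetVisibility call on Cube is left unconnected, so the flag never hides the mesh.
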(event `self.ReceiveBeginPlay`)

(event `self.ReceiveTick`
  (params (DeltaSeconds :type "Float (single-precision)"))
  (`KismetSystemLibrary.PrintString` (`KismetStringLibrary.Conv_BoolToString` (`OptimizerActorComponent.WasPrimitiveComponentRenderedRecently` (`self.OptimizerActor`) (`self.Cube`) 0.2)) true false (struct :`R` 1.0 :`G` 0.950846 :`A` 1.0) 0.0)
  (`KismetSystemLibrary.PrintString` (`KismetStringLibrary.Conv_BoolToString` (`self.Visible`)) true false (struct :`R` 0.279998 :`G` 1.0 :`B` 0.022275 :`A` 1.0) 0.0))

(event `self.OptimizerActor.OnCheckVisible`
  (params (VisibleFlag :type Boolean))
  (bind _output_get (set `self.Visible` VisibleFlag))
  (`KismetSystemLibrary.PrintString` (`KismetTextLibrary.Conv_TextToString` (`|FormatText` "[ Visible = {Visible} ] {Name} {timecode}" _output_get (`KismetSystemLibrary.GetObjectName` self) (`GameplayStatics.GetTimeSeconds`))) true false))

(fn `UserConstructionScript`)